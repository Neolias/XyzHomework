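; Base moving platform that drives its timeline forward and back in either Loop or OnDemand behavior.
; In Loop, BeginPlay starts alternating play and reverse calls chained by MovementCooldown timers, independent of timeline completion.
; In OnDemand, an XyzBaseCharacter entering the collision plays the timeline, and leaving schedules a reverse after the cooldown.
; The timer is not cleared on re-entry, and movement itself is defined outside these graphs.
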(event OnComponentEndOverlap(PlatformCollision)
  (params (OverlappedComponent :type Primitive%20Component%20Object%20Reference) (OtherActor :type Actor%20Object%20Reference) (OtherComp :type Primitive%20Component%20Object%20Reference) (OtherBodyIndex :type Integer))
  ;[1 0.2604 0.2604] On Demand Movement Logic
  (Utilities|Casting|CastToXyzBaseCharacter OtherActor)
  (if (Utilities|Enum|Equal(Enum) (Variables|Default|GetPlatformBehavior) "OnDemand")
    (Utilities|Time|SetTimerbyEvent (delegate Custom|OnPlatformReachedEndLocation2) (Variables|Default|GetMovementCooldown))))

(event OnComponentBeginOverlap(PlatformCollision)
  (params (OverlappedComponent :type Primitive%20Component%20Object%20Reference) (OtherActor :type Actor%20Object%20Reference) (OtherComp :type Primitive%20Component%20Object%20Reference) (OtherBodyIndex :type Integer) (bFromSweep :type Boolean) (SweepResult :type Hit%20Result%20Structure%20%28by%20ref%29))
  ;[1 0.2604 0.2604] On Demand Movement Logic
  (Utilities|Casting|CastToXyzBaseCharacter OtherActor)
  (if (Utilities|Enum|Equal(Enum) (Variables|Default|GetPlatformBehavior) "OnDemand")
    (Class|BasePlatform|PlatformTimelinePlay)))

(event Custom|OnPlatformReachedStartLocation
  ;[1 0.9206 0.202] Loop Movement Logic
  (Class|BasePlatform|PlatformTimelinePlay)
  (Utilities|Time|SetTimerbyEvent (delegate Custom|OnPlatformReachedEndLocation) (Variables|Default|GetMovementCooldown)))

(event Custom|OnPlatformReachedEndLocation2
  ;[1 0.2604 0.2604] On Demand Movement Logic
  (Class|BasePlatform|PlatformTimelineReverse))

(event Custom|OnPlatformReachedEndLocation
  ;[1 0.9206 0.202] Loop Movement Logic
  (Class|BasePlatform|PlatformTimelineReverse)
  (Utilities|Time|SetTimerbyEvent (delegate Custom|OnPlatformReachedStartLocation) (Variables|Default|GetMovementCooldown)))

(event EventBeginPlay
  ;[1 0.9206 0.202] Loop Movement Logic
  (if (Utilities|Enum|Equal(Enum) (Variables|Default|GetPlatformBehavior) "Loop")
    (Class|BasePlatform|PlatformTimelinePlay)
    (Utilities|Time|SetTimerbyEvent (delegate Custom|OnPlatformReachedEndLocation) (Variables|Default|GetMovementCooldown))))

(fn ConstructionScript)