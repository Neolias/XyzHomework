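; BP_Player is the player character Blueprint that changes the camera spring arm length while the player sprints.
; BeginPlay caches the default arm length, and the sprint start and stop events call their parent implementations before driving a timeline.
; The timeline lerps the arm between the default and sprint lengths, playing on start and reversing on stop for a smooth transition both ways.
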(event EventOnSprintStart
  (|CallParentFunction)
  (bind _newtrack_0 (Timeline|Sprint%20Arm%20Sprint%20Timeline Play)
    (:Update
      (Variables|/Script/Engine.SpringArmComponent|SetTargetArmLength (Variables|Default|GetSpringArmComponent) (Math|Float|Lerp (Variables|SprintSettings|GetDefaultArmLength) (Variables|SprintSettings|GetSpringArmLength) _newtrack_0)))))

(event EventOnSprintStop
  (|CallParentFunction)
  (bind _newtrack_0 (Timeline|Sprint%20Arm%20Sprint%20Timeline Reverse)
    (:Update
      (Variables|/Script/Engine.SpringArmComponent|SetTargetArmLength (Variables|Default|GetSpringArmComponent) (Math|Float|Lerp (Variables|SprintSettings|GetDefaultArmLength) (Variables|SprintSettings|GetSpringArmLength) _newtrack_0)))))

(event EventBeginPlay
  (Variables|SprintSettings|SetDefaultArmLength (Variables|/Script/Engine.SpringArmComponent|GetTargetArmLength (Variables|Default|GetSpringArmComponent))))

(fn ConstructionScript)